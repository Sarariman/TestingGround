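; AI controller for guard NPCs that runs the GuardBehaviour tree on a PatrolData blackboard.
; Perception updates store a sensed actor without the "Enemy" tag in the EnemyKey blackboard value and clear it when sensing is lost.
; Every tick it sets the controlled character's Aiming and Shooting flags according to whether the controller has a valid focus actor.
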(event `self.ReceiveBeginPlay`
  (bind _blackboardcomponent (`self.UseBlackboard` "/Game/Character/AI/PatrolData.PatrolData"))
  (`self.RunBehaviorTree` "/Game/Character/AI/GuardBehaviour.GuardBehaviour")
  (set `self.BlackboardComp` _blackboardcomponent))

(event `self.AIPerception.OnTargetPerceptionUpdated`
  (params (Actor :type "Actor Object Reference") (Stimulus :type "AIStimulus Structure"))
  (if (`self.ActorHasTag` Actor "Enemy")
    _
    (elif (`.bSuccessfullySensed` (break `AIStimulus` Stimulus))
      (`BlackboardComponent.SetValueAsObject` (`self.BlackboardComp`) (`self.EnemyKey`) Actor)
      (else
        ;[1 1 1] To Clear "Enemy" Key
        (`BlackboardComponent.ClearValue` (`self.BlackboardComp`) (`self.EnemyKey`))))))

(event `self.ReceiveTick`
  (params (DeltaSeconds :type "Float (single-precision)"))
  (bind _returnvalue (`KismetSystemLibrary.IsValid` (`self.GetFocusActor`)))
  (bind _ascharacter (cast `/Game/Character/Behaviour/Character` (`self.K2_GetPawn`)))
  (set `/Game/Character/Behaviour/Character.Aiming` _returnvalue _ascharacter)
  (set `/Game/Character/Behaviour/Character.Shooting` _returnvalue _ascharacter))

(fn `UserConstructionScript`)